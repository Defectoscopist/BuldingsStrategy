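; BP_BuildingParent is the base building actor, with working and trouble states that it reports to a BP_CellManager.
; Its construction script applies a height offset and creates dynamic material instances for its static meshes.
; AwakeTrouble flags trouble and restarts a timeline on finish to repeatedly lerp the materials from their stored color toward red.
; StopTroubles restores that color, and both events have the manager check the building group's system.
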(event Custom|AwakeTrouble
  (Variables|Default|SetbIsWorking false)
  (Variables|Default|SetbIsTrouble true)
  (Default|CheckSystemOfGroup (Variables|Default|GetCellManager) (Variables|Default|GetGroupNumber))
  (bind _returnvalue (Rendering|Material|GetVectorParameterValue (Utilities|Array|Get(acopy) (Variables|Default|GetDynamicMaterials)) "Param" :!class /Script/Engine.MaterialInstanceDynamic))
  (Variables|Default|SetStartMaterial _returnvalue)
  (bind _color (Timeline|ChangeColor PlayFromStart)
    (:Update
      (for _array_element (Variables|Default|GetDynamicMaterials)
        (Rendering|Material|SetVectorParameterValue _array_element "Param" (Math|Color|Lerp(LinearColor) (Variables|Default|GetStartMaterial) "(R=1.000000,G=0.000000,B=0.000000,A=1.000000)" _color) :!class /Script/Engine.MaterialInstanceDynamic)))
    (:Finished
      (Timeline|ChangeColor PlayFromStart))))

(event Custom|StopTroubles
  (Variables|Default|SetbIsWorking true)
  (Variables|Default|SetbIsTrouble false)
  (Utilities|FlowControl|Sequence
    (:then_0
      (bind _color (Timeline|ChangeColor Stop)
        (:Update
          (for _array_element (Variables|Default|GetDynamicMaterials)
            (Rendering|Material|SetVectorParameterValue _array_element "Param" (Math|Color|Lerp(LinearColor) (Variables|Default|GetStartMaterial) "(R=1.000000,G=0.000000,B=0.000000,A=1.000000)" _color) :!class /Script/Engine.MaterialInstanceDynamic)))
        (:Finished
          (Timeline|ChangeColor PlayFromStart))))
    (:then_1
      (for _array_element_2 (Variables|Default|GetDynamicMaterials)
        (Rendering|Material|SetVectorParameterValue _array_element_2 "Param" (Variables|Default|GetStartMaterial) :!class /Script/Engine.MaterialInstanceDynamic))
      (Default|CheckSystemOfGroup (Variables|Default|GetCellManager) (Variables|Default|GetGroupNumber)))))

(event Collision|EventActorBeginOverlap
  (params (OtherActor :type Actor%20Object%20Reference)))

(event EventTick
  (params (DeltaSeconds :type Float%20%28single-precision%29)))

(event EventBeginPlay
  (bind _outactors (Actor|GetAllActorsOfClass "/Game/Blueprints/Gameplay/BuildingCore/BP_CellManager.BP_CellManager_C"))
  (for _array_element _outactors
    (Variables|Default|SetCellManager _array_element)))

(fn ConstructionScript
  (bind _building (Variables|Default|GetBuilding))
  (bind _relativelocation (Variables|/Script/Engine.SceneComponent|GetRelativeLocation _building))
  (Transformation|SetRelativeLocation _building (Math|Vector|MakeVector (.x _relativelocation) (.y _relativelocation) (Variables|Default|GetZ_Offset)) false false)
  (for _array_element (Actor|GetComponentsByClass "/Script/Engine.StaticMeshComponent")
    (bind _returnvalue (Rendering|Material|CreateDynamicMaterialInstance _array_element 0 (Variables|Default|GetMaterial) "None" :!class /Script/Engine.PrimitiveComponent))
    (Utilities|Array|Add (Variables|Default|GetDynamicMaterials) _returnvalue)))