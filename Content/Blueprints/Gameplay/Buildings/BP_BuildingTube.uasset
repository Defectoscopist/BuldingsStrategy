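; BP_BuildingTube is a tube building that shows connecting segments toward occupied neighbouring grid cells.
; RotateTubes checks the cell's four neighbours for buildings and toggles segment visibility rather than rotating: Up drives DownTube, Down UpTube, Left RightTube, Right the Building component.
; BlankLeft and BlankRight show only when no segment is visible.
; Unlike the other segments, UpTube is never hidden again, as its hide call is unconnected.
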(event EventBeginPlay
  (|CallParentFunction) ; This node is disabled and will not be called.\nDrag off pins to build functionality.
)

(event Collision|EventActorBeginOverlap
  (params (OtherActor :type Actor%20Object%20Reference))
  (|CallParentFunction OtherActor) ; This node is disabled and will not be called.\nDrag off pins to build functionality.
)

(event EventTick
  (params (DeltaSeconds :type Float%20%28single-precision%29))
  (|CallParentFunction DeltaSeconds) ; This node is disabled and will not be called.\nDrag off pins to build functionality.
)

(fn ConstructionScript
  (|CallParentFunction))

(fn RotateTubes
  (params (Cell :type BP%20Plant%20Cell%20Object%20Reference))
  (bind _downtube (Variables|Default|GetDownTube))
  (bind _building (Variables|Default|GetBuilding))
  (bind _righttube (Variables|Default|GetRightTube))
  (Utilities|FlowControl|Sequence
    (:then_0
      (bind _upneighbour (Variables|/Game/Blueprints/Gameplay/BuildingCore/BP_PlantCell.BP_PlantCell_C|GetUpNeighbour Cell)
        (:then
          (if (Variables|/Game/Blueprints/Gameplay/BuildingCore/BPC_ClickableComponent.BPC_ClickableComponent_C|GetbHasBuilding (Variables|/Game/Blueprints/Gameplay/BuildingCore/BP_PlantCell.BP_PlantCell_C|GetClickableComponent _upneighbour))
            (Rendering|SetVisibility _downtube true false)
            (Rendering|SetVisibility (Variables|Default|GetBlankLeft) false false)
            (else
              (Rendering|SetVisibility _downtube false false))))
        (:else)))
    (:then_1
      (bind _downneighbour (Variables|/Game/Blueprints/Gameplay/BuildingCore/BP_PlantCell.BP_PlantCell_C|GetDownNeighbour Cell)
        (:then
          (if (Variables|/Game/Blueprints/Gameplay/BuildingCore/BPC_ClickableComponent.BPC_ClickableComponent_C|GetbHasBuilding (Variables|/Game/Blueprints/Gameplay/BuildingCore/BP_PlantCell.BP_PlantCell_C|GetClickableComponent _downneighbour))
            (Rendering|SetVisibility (Variables|Default|GetUpTube) true false)
            (Rendering|SetVisibility (Variables|Default|GetBlankLeft) false false)))
        (:else)))
    (:then_2
      (bind _leftneighbour (Variables|/Game/Blueprints/Gameplay/BuildingCore/BP_PlantCell.BP_PlantCell_C|GetLeftNeighbour Cell)
        (:then
          (if (Variables|/Game/Blueprints/Gameplay/BuildingCore/BPC_ClickableComponent.BPC_ClickableComponent_C|GetbHasBuilding (Variables|/Game/Blueprints/Gameplay/BuildingCore/BP_PlantCell.BP_PlantCell_C|GetClickableComponent _leftneighbour))
            (Rendering|SetVisibility _righttube true false)
            (Rendering|SetVisibility (Variables|Default|GetBlankLeft) false false)
            (else
              (Rendering|SetVisibility _righttube false false))))
        (:else)))
    (:then_3
      (bind _rightneighbour (Variables|/Game/Blueprints/Gameplay/BuildingCore/BP_PlantCell.BP_PlantCell_C|GetRightNeighbour Cell)
        (:then
          (if (Variables|/Game/Blueprints/Gameplay/BuildingCore/BPC_ClickableComponent.BPC_ClickableComponent_C|GetbHasBuilding (Variables|/Game/Blueprints/Gameplay/BuildingCore/BP_PlantCell.BP_PlantCell_C|GetClickableComponent _rightneighbour))
            (Rendering|SetVisibility _building true false)
            (Rendering|SetVisibility (Variables|Default|GetBlankLeft) false false)
            (else
              (Rendering|SetVisibility _building false false))))
        (:else)))
    (:then_4
      (if (Math|Boolean|ORBoolean (Variables|/Script/Engine.SceneComponent|GetbVisible (Variables|Default|GetRightTube)) (Variables|/Script/Engine.SceneComponent|GetbVisible (Variables|Default|GetDownTube)) (Variables|/Script/Engine.SceneComponent|GetbVisible (Variables|Default|GetUpTube)) (Variables|/Script/Engine.SceneComponent|GetbVisible (Variables|Default|GetBuilding)))
        (Rendering|SetVisibility (Variables|Default|GetBlankLeft) false false)
        (else
          (Rendering|SetVisibility (Variables|Default|GetBlankLeft) true false))))))