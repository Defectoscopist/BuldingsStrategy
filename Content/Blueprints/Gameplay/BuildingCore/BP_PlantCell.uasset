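; BP_PlantCell is a cell actor that dresses itself at BeginPlay with either a stone or random plants.
; On a rare roll it reveals its stone mesh with random offset, yaw and scale and sets HasStone.
; Otherwise it destroys the stone and uses coin-flip loops to attach one or more of each plant type at random positions.
; Spawned plants are stored in an array for DestroyPlants to clear, while FindYourNeighbour is an empty stub.
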(event EventBeginPlay
  (if (< (Math|Random|RandomFloatinRange 0.0 1.0) 0.1)
    (CallFunction|SpawnStone)
    (else
      (CallFunction|SpawnPlants))))

(event Collision|EventActorBeginOverlap
  (params (OtherActor :type Actor%20Object%20Reference)))

(event EventTick
  (params (DeltaSeconds :type Float%20%28single-precision%29))
  ;[1 1 1] Group Debug
)

(fn ConstructionScript)

(fn SpawnStone
  (bind _returnvalue (Math|Random|RandomFloatinRange 1.0 2.0))
  (bind _sm_stone (Variables|Default|GetSM_Stone))
  (Transformation|SetRelativeTransform _sm_stone (Math|Transform|MakeTransform (Math|Vector|MakeVector (Math|Random|RandomFloatinRange -1.3e+02 1.3e+02) (Math|Random|RandomFloatinRange -1.8e+02 1.8e+02) 7e+01) (Math|Rotator|MakeRotator 0.0 0.0 (Math|Random|RandomFloatinRange 0.0 3.6e+02)) (Math|Vector|MakeVector _returnvalue _returnvalue _returnvalue)) false false)
  (Rendering|SetVisibility _sm_stone true false)
  (Variables|Default|SetHasStone true))

(fn SpawnPlants
  (Components|DestroyComponent (Variables|Default|GetSM_Stone))
  (bind _returnvalue (Game|SpawnActorfromClass "/Game/Blueprints/Landscape/BP_Plant1.BP_Plant1_C" (Math|Transform|MakeTransform "0, 0, 0" "0, 0, 0" "1,1,1") "Undefined" self 0 :!label _label))
  (Utilities|Array|Add (Variables|Default|GetPlants) _returnvalue)
  (Transformation|AttachActorToActor _returnvalue self "None" "KeepRelative" "KeepRelative" "KeepRelative" true)
  (Transformation|SetActorRelativeTransform _returnvalue (Math|Transform|MakeTransform (Math|Vector|MakeVector (Math|Random|RandomFloatinRange -2e+02 2e+02) (Math|Random|RandomFloatinRange -2e+02 2e+02) 0.0) (Math|Rotator|MakeRotator 0.0 0.0 (Math|Random|RandomFloatinRange 0.0 3.6e+02)) "1,1,1") false false)
  (if (< (Math|Random|RandomFloatinRange 0.0 1.0) 0.5)
    (goto _label)
    (else
      (bind _returnvalue_2 (Game|SpawnActorfromClass "/Game/Blueprints/Landscape/BP_Plant2.BP_Plant2_C" (Math|Transform|MakeTransform "0, 0, 0" "0, 0, 0" "1,1,1") "Undefined" self 0 :!label _label_2))
      (Utilities|Array|Add (Variables|Default|GetPlants) _returnvalue_2)
      (Transformation|AttachActorToActor _returnvalue_2 self "None" "KeepRelative" "KeepRelative" "KeepRelative" true)
      (Transformation|SetActorRelativeTransform _returnvalue_2 (Math|Transform|MakeTransform (Math|Vector|MakeVector (Math|Random|RandomFloatinRange -2e+02 2e+02) (Math|Random|RandomFloatinRange -2e+02 2e+02) 0.0) (Math|Rotator|MakeRotator 0.0 0.0 (Math|Random|RandomFloatinRange 0.0 3.6e+02)) "1,1,1") false false)
      (if (< (Math|Random|RandomFloatinRange 0.0 1.0) 0.5)
        (goto _label_2)))))

(fn DestroyPlants
  (bind _plants (Variables|Default|GetPlants))
  (bind _arrayelement (Utilities|Array|ReverseforEachLoop _plants)
    (:LoopBody
      (Utilities|IsValid _arrayelement
        (:Is%20Valid
          (Actor|DestroyActor _arrayelement))))
    (:Completed
      (Utilities|Array|Clear _plants))))

(fn FindYourNeighbour
  (params (ItsIndex :type Integer)))