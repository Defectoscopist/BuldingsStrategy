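; Manager for a building game that spawns a 20x20 grid of BP_PlantCell actors, links their neighbours and runs the resource economy.
; A looping timer adds Money, Oil and Water from working groups, rebuilds Food and Power from a per-building map, then updates the HUD.
; CheckSystemOfGroup marks a group working when it has all five building types untroubled.
; MakeTrouble breaks a random building and sends job-matched workers to repair it.
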(event Custom|CalculateResources
  (bind _building_resource (Variables|Default|GetBuilding_Resource))
  (bind _outactors (Actor|GetAllActorsOfClass "/Game/Blueprints/Gameplay/Buildings/BP_BuildingParent.BP_BuildingParent_C"))
  (for _array_element _outactors
    (if (Variables|/Game/Blueprints/Gameplay/Buildings/BP_BuildingParent.BP_BuildingParent_C|GetbIsTrouble _array_element)
      (if (.ReturnValue (Utilities|Map|Find _building_resource _array_element)) :!label _label
        (Utilities|Map|Add _building_resource _array_element 0))
      (elif (.ReturnValue (Utilities|Map|Find (Variables|Default|GetGroup_Works) (Variables|/Game/Blueprints/Gameplay/Buildings/BP_BuildingParent.BP_BuildingParent_C|GetGroupNumber _array_element)))
        (if (.Value (Utilities|Map|Find (Variables|Default|GetGroup_Works) (Variables|/Game/Blueprints/Gameplay/Buildings/BP_BuildingParent.BP_BuildingParent_C|GetGroupNumber _array_element)))
          (switch Utilities|FlowControl|Switch|SwitchonE_TypeOfBuilding (Variables|/Game/Blueprints/Gameplay/Buildings/BP_BuildingParent.BP_BuildingParent_C|GetTypeOfBuilding _array_element)
            (:NewEnumerator0
              (Variables|Resources|SetMoney (+ (Variables|Resources|GetMoney) 50)))
            (:NewEnumerator1
              (Utilities|Map|Add (Variables|Default|GetBuilding_Resource) _array_element 1000))
            (:NewEnumerator2
              (Utilities|Map|Add (Variables|Default|GetBuilding_Resource) _array_element 500))
            (:NewEnumerator3
              (Variables|Resources|SetOil (+ (Variables|Resources|GetOil) 10)))
            (:NewEnumerator4
              (Variables|Resources|SetWater (+ (Variables|Resources|GetWater) 20))))
          (else
            (goto _label))))))
  (Variables|Resources|SetFood 0)
  (Variables|Resources|SetPower 0)
  (bind _outactors_2 (Actor|GetAllActorsOfClass "/Game/Blueprints/Gameplay/Buildings/BP_BuildingDining.BP_BuildingDining_C"))
  (for _array_element_2 _outactors_2
    (if (.ReturnValue (Utilities|Map|Find (Variables|Default|GetBuilding_Resource) _array_element_2))
      (Variables|Resources|SetFood (+ (.Value (Utilities|Map|Find (Variables|Default|GetBuilding_Resource) _array_element_2)) (Variables|Resources|GetFood)))))
  (bind _outactors_3 (Actor|GetAllActorsOfClass "/Game/Blueprints/Gameplay/Buildings/BP_BuildingPowerPlant.BP_BuildingPowerPlant_C"))
  (for _array_element_3 _outactors_3
    (if (.ReturnValue (Utilities|Map|Find (Variables|Default|GetBuilding_Resource) _array_element_3))
      (Variables|Resources|SetPower (+ (.Value (Utilities|Map|Find (Variables|Default|GetBuilding_Resource) _array_element_3)) (Variables|Resources|GetPower)))))
  (Default|UpdateResources (Variables|/Game/Blueprints/Gameplay/UI/MainHUD.MainHUD_C|GetPlayerUI (Variables|Default|GetAs%20Main%20HUD))))

(event EventBeginPlay
  (bind _cells (Variables|Default|GetCells))
  (Utilities|Time|SetTimerbyEvent (delegate Custom|CalculateResources) 5.0 true)
  (bind _asmain_hud (Utilities|Casting|CastToMainHUD (HUD|GetHUD (Game|GetPlayerController 0))))
  (Variables|Default|SetAs%20Main%20HUD _asmain_hud)
  (while (<= (Utilities|Array|Length (Variables|Default|GetCells)) 399)
    (bind _returnvalue (Game|SpawnActorfromClass "/Game/Blueprints/Gameplay/BuildingCore/BP_PlantCell.BP_PlantCell_C" (Math|Transform|MakeTransform (Variables|Default|GetSpawnLocation_0) "0, 0, 0" "1,1,1") "AlwaysSpawn" 0 0))
    (Transformation|SetWorldLocation (Variables|/Game/Blueprints/Gameplay/BuildingCore/BP_PlantCell.BP_PlantCell_C|GetDefaultSceneRoot _returnvalue) (Variables|Default|GetSpawnLocation_0) false false)
    (Utilities|Array|AddUnique _cells _returnvalue)
    (if (== (Math|Integer|%(Integer) (Utilities|Array|Length _cells) 20) 0)
      (Variables|Default|SetSpawnLocation_0 (Math|Vector|MakeVector (+ (.x (Variables|Default|GetSpawnLocation_0)) 1e+03) (- (.y (Variables|Default|GetSpawnLocation_0)) 1.9e+04) 0.0))
      (else
        (Variables|Default|SetSpawnLocation_0 (Math|Vector|MakeVector (.x (Variables|Default|GetSpawnLocation_0)) (+ (.y (Variables|Default|GetSpawnLocation_0)) 1e+03) 0.0)))))
  (for (_array_element _array_index) (Variables|Default|GetCells)
    (Variables|Default|SetArray%20Index _array_index)
    (CallFunction|SetLeftNeighbour _array_element)
    (CallFunction|SetRightNeighbour _array_element)
    (CallFunction|SetUpNeighbour _array_element)
    (CallFunction|SetDownNeighbour _array_element)))

(fn ConstructionScript)

(fn SetLeftNeighbour
  (params (Cell :type BP%20Plant%20Cell%20Object%20Reference))
  (if (Utilities|Array|IsValidIndex (Variables|Default|GetCells) (- (Variables|Default|GetArray%20Index) 1))
    (if (!= (Math|Integer|%(Integer) (- (Variables|Default|GetArray%20Index) 1) 20) 19)
      (Variables|/Game/Blueprints/Gameplay/BuildingCore/BP_PlantCell.BP_PlantCell_C|SetLeftNeighbour Cell (Utilities|Array|Get(acopy) (Variables|Default|GetCells) (- (Variables|Default|GetArray%20Index) 1))))))

(fn SetRightNeighbour
  (params (Cell :type BP%20Plant%20Cell%20Object%20Reference))
  (if (Utilities|Array|IsValidIndex (Variables|Default|GetCells) (+ (Variables|Default|GetArray%20Index) 1))
    (if (!= (Math|Integer|%(Integer) (+ (Variables|Default|GetArray%20Index) 1) 20) 0)
      (Variables|/Game/Blueprints/Gameplay/BuildingCore/BP_PlantCell.BP_PlantCell_C|SetRightNeighbour Cell (Utilities|Array|Get(acopy) (Variables|Default|GetCells) (+ (Variables|Default|GetArray%20Index) 1))))))

(fn SetUpNeighbour
  (params (Cell :type BP%20Plant%20Cell%20Object%20Reference))
  (if (Utilities|Array|IsValidIndex (Variables|Default|GetCells) (+ (Variables|Default|GetArray%20Index) 20))
    (Variables|/Game/Blueprints/Gameplay/BuildingCore/BP_PlantCell.BP_PlantCell_C|SetUpNeighbour Cell (Utilities|Array|Get(acopy) (Variables|Default|GetCells) (+ (Variables|Default|GetArray%20Index) 20)))))

(fn SetDownNeighbour
  (params (Cell :type BP%20Plant%20Cell%20Object%20Reference))
  (if (Utilities|Array|IsValidIndex (Variables|Default|GetCells) (- (Variables|Default|GetArray%20Index) 20))
    (Variables|/Game/Blueprints/Gameplay/BuildingCore/BP_PlantCell.BP_PlantCell_C|SetDownNeighbour Cell (Utilities|Array|Get(acopy) (Variables|Default|GetCells) (- (Variables|Default|GetArray%20Index) 20)))))

(fn CalculateResource
  (params (Add/Minus :type Integer) (Resource :type E_TypeOfResource%20Enum :default "NewEnumerator0"))
  (Utilities|FlowControl|Sequence
    (:then_0
      (switch Utilities|FlowControl|Switch|SwitchonE_TypeOfResource Resource
        (:NewEnumerator0
          (Variables|Resources|SetMoney (+ (Variables|Resources|GetMoney) Add/Minus)))
        (:NewEnumerator1
          (Variables|Resources|SetWater (+ (Variables|Resources|GetWater) Add/Minus)))
        (:NewEnumerator2
          (Variables|Resources|SetFood (+ (Variables|Resources|GetFood) Add/Minus)))
        (:NewEnumerator3
          (Variables|Resources|SetPower (+ (Variables|Resources|GetPower) Add/Minus)))
        (:NewEnumerator4
          (Variables|Resources|SetOil (+ (Variables|Resources|GetOil) Add/Minus)))))
    (:then_1
      (Default|UpdateResources (Variables|/Game/Blueprints/Gameplay/UI/MainHUD.MainHUD_C|GetPlayerUI (Variables|Default|GetAs%20Main%20HUD))))))

(fn MakeTrouble
  (bind _outactors (Actor|GetAllActorsOfClass "/Game/Blueprints/Gameplay/Buildings/BP_BuildingParent.BP_BuildingParent_C"))
  (bind _output_get (Variables|Default|SetBuildings _outactors))
  (if (!= (Utilities|Array|Length _output_get) 0)
    (Utilities|Array|Shuffle _output_get)
    (Default|AwakeTrouble (Utilities|Array|Get(acopy) _output_get))
    (bind _output_get_2 (Variables|Default|SetTroubleBuilding (Utilities|Array|Get(acopy) _output_get)))
    (bind _outactors_2 (Actor|GetAllActorsOfClass "/Game/Blueprints/Gameplay/Workers/BP_Worker.BP_Worker_C"))
    (for _array_element _outactors_2
      (if (Utilities|Enum|Equal(Enum) (Variables|/Game/Blueprints/Gameplay/Workers/BP_Worker.BP_Worker_C|GetJob _array_element) (Variables|/Game/Blueprints/Gameplay/Buildings/BP_BuildingParent.BP_BuildingParent_C|GetTypeOfBuilding _output_get_2))
        (Default|RepairBuilding _array_element (Transformation|GetWorldLocation (Variables|/Game/Blueprints/Gameplay/Buildings/BP_BuildingParent.BP_BuildingParent_C|GetBuilding (Variables|Default|GetTroubleBuilding))))))))

(fn CancelTrouble
  (bind _troublebuilding (Variables|Default|GetTroubleBuilding)
    (:then
      (Default|StopTroubles _troublebuilding)
      (Variables|Default|SetTroubleBuilding 0))
    (:else)))

(fn CheckSystemOfGroup
  (params (GroupNumber :type Integer))
  (bind _checktypes (Variables|Default|GetCheckTypes))
  (bind _returnvalue (Utilities|Array|Length _checktypes))
  (bind _returnvalue_2 (>= _returnvalue 5))
  (bind _outactors (Actor|GetAllActorsOfClass "/Game/Blueprints/Gameplay/Buildings/BP_BuildingParent.BP_BuildingParent_C"))
  (for _array_element _outactors
    (if (== (Variables|/Game/Blueprints/Gameplay/Buildings/BP_BuildingParent.BP_BuildingParent_C|GetGroupNumber _array_element) GroupNumber)
      (if (not (Variables|/Game/Blueprints/Gameplay/Buildings/BP_BuildingParent.BP_BuildingParent_C|GetbIsTrouble _array_element))
        (switch Utilities|FlowControl|Switch|SwitchonE_TypeOfBuilding (Variables|/Game/Blueprints/Gameplay/Buildings/BP_BuildingParent.BP_BuildingParent_C|GetTypeOfBuilding _array_element)
          (:NewEnumerator0
            _)
          (:NewEnumerator1
            _)
          (:NewEnumerator2
            _)
          (:NewEnumerator3
            _)
          (:NewEnumerator4
            _))
        (Utilities|Array|AddUnique (Variables|Default|GetCheckTypes) (Variables|/Game/Blueprints/Gameplay/Buildings/BP_BuildingParent.BP_BuildingParent_C|GetTypeOfBuilding _array_element)))))
  (Utilities|Map|Add (Variables|Default|GetGroup_Works) GroupNumber _returnvalue_2)
  (bind _outactors_2 (Actor|GetAllActorsOfClass "/Game/Blueprints/Gameplay/Buildings/BP_BuildingParent.BP_BuildingParent_C"))
  (for _array_element_2 _outactors_2
    (if (== (Variables|/Game/Blueprints/Gameplay/Buildings/BP_BuildingParent.BP_BuildingParent_C|GetGroupNumber _array_element_2) GroupNumber)
      (Variables|/Game/Blueprints/Gameplay/Buildings/BP_BuildingParent.BP_BuildingParent_C|SetbIsWorking _array_element_2 _returnvalue_2)
      (else
        (Variables|/Game/Blueprints/Gameplay/Buildings/BP_BuildingParent.BP_BuildingParent_C|SetbIsWorking _array_element_2 false))))
  (Utilities|Array|Clear (Variables|Default|GetCheckTypes)))