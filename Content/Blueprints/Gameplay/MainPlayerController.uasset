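; Player controller that routes input to a controlled CameraPawn for camera movement and exposes game-level shortcuts.
; BeginPlay caches the pawn, then movement, strafe and rotation axes forward directly to it, while the Zoom action passes the pressed key's axis value.
; Right mouse button calls OutBuildingMode on the GI_Building game instance, and Escape quits the game.
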(event EventBeginPlay
  (bind _ascamera_pawn (Utilities|Casting|CastToCameraPawn (Pawn|GetControlledPawn)))
  (Variables|Default|SetAs%20Main%20Camera%20Controller _ascamera_pawn))

(event Input|ActionEvents|InputActionZoom
  (params (Key :type Key%20Structure :default "None"))
  ;[1 1 1] Inputs
  (:Pressed
    (Default|CameraZoom (Variables|Default|GetAs%20Main%20Camera%20Controller) (Class|Actor|GetInputAxisKeyValue Key))))

(event Input|AxisEvents|InputAxisCameraRot
  (params (AxisValue :type Float%20%28single-precision%29))
  ;[1 1 1] Inputs
  (Default|CameraRotation (Variables|Default|GetAs%20Main%20Camera%20Controller) AxisValue))

(event Input|AxisEvents|InputAxisMoveForwardBacward
  (params (AxisValue :type Float%20%28single-precision%29))
  ;[1 1 1] Inputs
  (Default|MoveForwardBackward (Variables|Default|GetAs%20Main%20Camera%20Controller) AxisValue))

(event Input|AxisEvents|InputAxisStrafe
  (params (AxisValue :type Float%20%28single-precision%29))
  ;[1 1 1] Inputs
  (Default|Strafe (Variables|Default|GetAs%20Main%20Camera%20Controller) AxisValue))

(event Input|KeyboardEvents|Escape
  (params (Key :type Key%20Structure :default "None"))
  ;[1 1 1] Inputs
  (:Pressed
    (Game|QuitGame 0 "Quit" false)))

(event Input|MouseEvents|RightMouseButton
  (params (Key :type Key%20Structure :default "None"))
  ;[1 1 1] Inputs
  (:Pressed
    (bind _asgi_building (Utilities|Casting|CastToGI_Building (Game|GetGameInstance)))
    (Default|OutBuildingMode _asgi_building)))

(fn ConstructionScript)