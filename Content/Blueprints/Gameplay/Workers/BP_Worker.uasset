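; Worker owned by a BP_PlantCell that wanders around and can be sent to repair a building.
; A timeline lerps it through chained random diagonal steps; RepairBuilding interrupts this to walk it to the given location.
; On arrival it spins on a looping timer for a fixed delay, calls CancelTrouble on BP_CellManager, then resumes wandering.
; SetCloses stores its profession as Job and applies the matching material to its meshes.
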(event Custom|ChangeDirection
  (bind _defaultsceneroot (Variables|Default|GetDefaultSceneRoot))
  (bind _returnvalue (Transformation|GetWorldLocation _defaultsceneroot))
  (Variables|Default|SetFromWalkLocation _returnvalue)
  (if (Variables|Default|GetbIsRepairing)
    (bind _walk (Timeline|Timeline_0 PlayFromStart)
      (:Update
        (Transformation|SetWorldLocation (Variables|Default|GetDefaultSceneRoot) (Math|Vector|Lerp(Vector) (Variables|Default|GetFromWalkLocation) (Variables|Default|GetToWalkLocation) _walk) false false))
      (:Finished
        (if (Variables|Default|GetbIsRepairing)
          (bind _returnvalue_2 (Utilities|Time|SetTimerbyEvent (delegate Custom|RepairingProcess) 0.02 true))
          (bind _output_get (Variables|Default|SetRepairingTimer _returnvalue_2))
          (Utilities|FlowControl|Delay 5.0)
          (Utilities|Time|ClearandInvalidateTimerbyHandle _output_get)
          (Variables|Default|SetbIsRepairing false)
          (Default|CancelTrouble (Variables|Default|GetCellManager))
          (CallFunction|ChangeDirection)
          (else
            (CallFunction|ChangeDirection)))))
    (else
      (Variables|Default|SetToWalkLocation (+ _returnvalue (Math|Vector|MakeVector (Math|Float|SelectFloat 4.5e+02 -4.5e+02 (Math|Random|RandomBool)) (Math|Float|SelectFloat 4.5e+02 -4.5e+02 (Math|Random|RandomBool)) 0.0)))
      (Timeline|Timeline_0 PlayFromStart))))

(event Custom|RepairBuilding
  (params (BuildingLocation :type Vector))
  (Variables|Default|SetbIsRepairing true)
  (Utilities|FlowControl|Sequence
    (:then_0
      (bind _walk (Timeline|Timeline_0 Stop)
        (:Update
          (Transformation|SetWorldLocation (Variables|Default|GetDefaultSceneRoot) (Math|Vector|Lerp(Vector) (Variables|Default|GetFromWalkLocation) (Variables|Default|GetToWalkLocation) _walk) false false))
        (:Finished
          (if (Variables|Default|GetbIsRepairing)
            (bind _returnvalue (Utilities|Time|SetTimerbyEvent (delegate Custom|RepairingProcess) 0.02 true))
            (bind _output_get (Variables|Default|SetRepairingTimer _returnvalue))
            (Utilities|FlowControl|Delay 5.0)
            (Utilities|Time|ClearandInvalidateTimerbyHandle _output_get)
            (Variables|Default|SetbIsRepairing false)
            (Default|CancelTrouble (Variables|Default|GetCellManager))
            (CallFunction|ChangeDirection)
            (else
              (CallFunction|ChangeDirection))))))
    (:then_1
      (Variables|Default|SetToWalkLocation BuildingLocation)
      (CallFunction|ChangeDirection))))

(event Custom|RepairingProcess
  (Transformation|AddWorldRotation (Variables|Default|GetDefaultSceneRoot) "0,1.000000, 0" false false))

(event EventBeginPlay
  (bind _asbp_plant_cell (Utilities|Casting|CastToBP_PlantCell (Components|GetOwner)))
  (Variables|Default|SetHomeCell _asbp_plant_cell)
  (CallFunction|ChangeDirection)
  (bind _outactors (Actor|GetAllActorsOfClass "/Game/Blueprints/Gameplay/BuildingCore/BP_CellManager.BP_CellManager_C"))
  (for _array_element _outactors
    (Variables|Default|SetCellManager _array_element)))

(fn ConstructionScript)

(fn SetCloses
  (params (Profession :type E_TypeOfBuilding%20Enum :default "NewEnumerator0"))
  (bind _cylinder (Variables|Default|GetCylinder))
  (bind _sm_cube (Variables|Default|GetSM_Cube))
  (Utilities|FlowControl|Sequence
    (:then_0
      (switch Utilities|FlowControl|Switch|SwitchonE_TypeOfBuilding Profession
        (:NewEnumerator0
          (Rendering|Material|SetMaterial _cylinder 0 "/Game/Materials_Textures/Buildings/M_LivingHouse.M_LivingHouse"))
        (:NewEnumerator1
          (Rendering|Material|SetMaterial _cylinder 0 "/Game/Materials_Textures/Buildings/M_PowerPlant.M_PowerPlant"))
        (:NewEnumerator2
          (Rendering|Material|SetMaterial _cylinder 0 "/Game/Materials_Textures/Buildings/M_Dining.M_Dining"))
        (:NewEnumerator3
          (Rendering|Material|SetMaterial _sm_cube 0 "/Game/Materials_Textures/Buildings/M_OilWell.M_OilWell"))
        (:NewEnumerator4
          (Rendering|Material|SetMaterial _cylinder 0 "/Game/Materials_Textures/Buildings/M_WaterTower.M_WaterTower"))
        (:NewEnumerator6
          (Rendering|Material|SetMaterial _sm_cube 0 "/Game/Materials_Textures/Buildings/M_Tube.M_Tube" :!label _label))
        (:NewEnumerator5
          (goto _label))))
    (:then_1
      (bind _output_get (Variables|Default|SetJob Profession)))))