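; CameraPawn is a player-controlled camera pawn with movement, rotation and spring-arm zoom.
; Input events yaw the actor and move it along its forward and right vectors with swept world offsets.
; Scroll zoom runs a timeline that lerps the spring arm length toward a clamped target.
; A gate closes while the timeline updates and reopens when it finishes, blocking new zoom input mid-transition.
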(event Custom|CameraRotation
  (params (Yaw :type Float%20%28single-precision%29))
  ;[1 1 1] Camera Move
  ;;[0 0 0] Q/E
  (Transformation|AddActorLocalRotation (Math|Rotator|MakeRotator 0.0 0.0 (* Yaw 3.0)) false false))

(event Custom|Move%20ForwardBackward
  (params (Step :type Float%20%28single-precision%29))
  ;[1 1 1] Camera Move
  ;;[0 0 0] W/S
  (Transformation|AddActorWorldOffset (* (Transformation|GetActorForwardVector self) (* Step 1e+02)) true))

(event Custom|Strafe
  (params (Step :type Float%20%28single-precision%29))
  ;[1 1 1] Camera Move
  ;;[0 0 0] A/D
  (Transformation|AddActorWorldOffset (* (Transformation|GetActorRightVector self) (* Step 1e+02)) true))

(event Custom|CameraZoom
  (params (Zoom :type Float%20%28single-precision%29))
  ;[1 1 1] Camera Move
  ;;[0 0 0] Scroll
  (Utilities|FlowControl|Gate false :!label _label
    (:Exit
      (bind _newtrack_0 (Timeline|Timeline_0 PlayFromStart)
        (:Update
          (Variables|/Script/Engine.SpringArmComponent|SetTargetArmLength (Variables|Default|GetSpringArm) (Math|Float|Lerp (Variables|/Script/Engine.SpringArmComponent|GetTargetArmLength (Variables|Default|GetSpringArm)) (Math|Float|Clamp(Float) (+ (* Zoom (Variables|Default|GetZoomSpeed)) (Variables|/Script/Engine.SpringArmComponent|GetTargetArmLength (Variables|Default|GetSpringArm))) 3e+03 5e+03) _newtrack_0))
          (goto _label Close))
        (:Finished
          (goto _label Open))))))

(fn ConstructionScript)